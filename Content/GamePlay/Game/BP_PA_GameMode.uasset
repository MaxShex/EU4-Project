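; Game mode Blueprint that continuously spawns donut actors around the player during play.
; On BeginPlay it starts a looping one-second timer that calls the SpawnDonut function.
; Each call spawns a BP_Actor_Donut above player pawn 0, randomly offset on X and Y within a square centered on that pawn's current location.
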(event Custom|CustomEvent_0
  (CallFunction|SpawnDonut))

(event EventBeginPlay
  (Utilities|Time|SetTimerbyEvent (delegate Custom|CustomEvent_0) 1.0 true))

(event EventTick
  (params (DeltaSeconds :type Float%20%28single-precision%29)))

(fn ConstructionScript)

(fn SpawnDonut
  (bind _returnvalue (Game|Player|GetPlayerPawn 0))
  (bind _returnvalue_2 (Transformation|GetActorLocation _returnvalue))
  (Game|SpawnActorfromClass "/Game/GamePlay/Weather/BP_Actor_Donut.BP_Actor_Donut_C" (Math|Transform|MakeTransform (Math|Vector|MakeVector (+ (Math|Random|RandomFloatinRange -5e+02 5e+02) (.x _returnvalue_2)) (+ (.y _returnvalue_2) (Math|Random|RandomFloatinRange -5e+02 5e+02)) (+ (.z _returnvalue_2) 5e+02)) "0, 0, 0" "1,1,1") "Undefined" 0 0))