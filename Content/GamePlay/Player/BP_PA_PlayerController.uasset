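; BP_PA_PlayerController is a player controller that drives first-person or third-person style movement and look for BP_PA_Character.
; On possess it casts the pawn to BP_PA_Character and caches the reference.
; MoveForward and MoveRight axes feed movement input along the character's forward and right vectors, while LookUp and Turn add pitch and yaw input to the controller.
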(event EventPossess
  (params (PossessedPawn :type Pawn%20Object%20Reference))
  (bind _output_get (Variables|Default|SetPossessed%20Pawn PossessedPawn))
  (bind _asbp_pa_character (Utilities|Casting|CastToBP_PA_Character _output_get))
  (Variables|Default|SetBP%20PA%20Character _asbp_pa_character))

(event Input|AxisEvents|InputAxisMoveForward
  (params (AxisValue :type Float%20%28single-precision%29))
  (bind _bp_pa_character (Variables|Default|GetBP%20PA%20Character))
  ;[1 1 1] Moving
  (Pawn|Input|AddMovementInput _bp_pa_character (Transformation|GetActorForwardVector _bp_pa_character) AxisValue false))

(event Input|AxisEvents|InputAxisMoveRight
  (params (AxisValue :type Float%20%28single-precision%29))
  (bind _bp_pa_character (Variables|Default|GetBP%20PA%20Character))
  ;[1 1 1] Moving
  (Pawn|Input|AddMovementInput _bp_pa_character (Transformation|GetActorRightVector _bp_pa_character) AxisValue false))

(event Input|AxisEvents|InputAxisTurn
  (params (AxisValue :type Float%20%28single-precision%29))
  (Class|PlayerController|AddYawInput AxisValue))

(event Input|AxisEvents|InputAxisLookUp
  (params (AxisValue :type Float%20%28single-precision%29))
  (Class|PlayerController|AddPitchInput AxisValue))

(fn ConstructionScript)